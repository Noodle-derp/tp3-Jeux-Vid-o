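; Milk hose component for the player character that sprays milk projectiles and tracks the milk tank level, shown on the backpack gauge through a dynamic material.
; While aiming, IA_Clean drains milk over time and launches BP_Projectile_Lait from the nozzle socket along an arc toward the crosshair's world position, with an attached looping-guarded sound.
; RemplirLait refills at four times LaitPerSecond, and a debug key fills the tank instantly.
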(event Input|EnhancedActionEvents|EnhancedInputActionIA_Clean
  (params (ActionValue :type Boolean) (ElapsedSeconds :type Float%20%28double-precision%29) (TriggeredSeconds :type Float%20%28double-precision%29) (InputAction :type Input%20Action%20Object%20Reference :default "/Game/ThirdPerson/Input/Actions/IA_Clean.IA_Clean"))
  (bind _returnvalue (Transformation|GetSocketLocation "NozzleSocket"))
  ;[0.7917 0.7915 0.6106 0.5 64] Projectiles Lait
  (:Triggered
    (if (Variables|/Game/ThirdPerson/Blueprints/BP_ThirdPersonCharacter.BP_ThirdPersonCharacter_C|GetIsAiming (Variables|Default|GetReferencePawnJoueur))
      (bind _emtpy_ (CallFunction|UtiliserLait))
      (if (not _emtpy_)
        (Utilities|FlowControl|Sequence
          (:then_0
            (Utilities|FlowControl|DoOnce false :!label _label
              (:Completed
                (bind _returnvalue_2 (Audio|SpawnSoundAttached "/Game/Audio/SFX/Filling.Filling" self "NozzleSocket" _returnvalue "0, 0, 0" "KeepRelativeOffset" false 0.25 1.0 1.0 0 0))
                (Variables|Default|SetSoundFX _returnvalue_2))))
          (:then_1
            (bind _outlaunchvelocity (Game|SuggestProjectileVelocityCustomArc _returnvalue (Variables|/Game/ThirdPerson/Blueprints/BP_ThirdPersonCharacter.BP_ThirdPersonCharacter_C|GetPositionMondeDeLaMire (Variables|Default|GetReferencePawnJoueur)) 0.0 (Variables|Default|GetArc%20Projectile%20Lait)))
            (bind _returnvalue_3 (Game|SpawnActorfromClass "/Game/Blueprint/Projectiles/BP_Projectile_Lait.BP_Projectile_Lait_C" (Math|Transform|MakeTransform _returnvalue (Variables|Default|GetNozzleRotation)) "Undefined" "MultiplyWithRoot" 0 0))
            (Variables|/Script/Engine.MovementComponent|SetVelocity (Variables|/Game/Blueprint/Projectiles/BP_Projectile.BP_Projectile_C|GetProjectileMovement _returnvalue_3) _outlaunchvelocity)))
        (else
          (Utilities|IsValid (Variables|Default|GetSoundFX) :!label _label_2
            (:Is%20Valid
              (Audio|Components|Audio|Stop (Variables|Default|GetSoundFX))
              (goto _label Reset)))))))
  (:Canceled
    (goto _label_2))
  (:Completed
    (goto _label_2)))

(event EventBeginPlay
  ;[0.15 0.15 0.15 0.5] Création d'un matériel dynamique pour la jauge du lait
  (bind _returnvalue (Rendering|Material|CreateDynamicMaterialInstance 1 "/Game/Art/Materials/MI_JaugeLait.MI_JaugeLait" "None" :!class /Script/Engine.PrimitiveComponent))
  (Variables|Default|SetM_JaugeLait_Reference _returnvalue)
  (bind _asbp_third_person_character (Utilities|Casting|CastToBP_ThirdPersonCharacter (Components|GetOwner)))
  (Variables|Default|SetReferencePawnJoueur _asbp_third_person_character))

(event EventTick
  (params (DeltaSeconds :type Float%20%28single-precision%29))
  (bind _jauge_lait_actuel (Variables|Default|GetJauge%20Lait%20Actuel))
  (bind _jauge_lait_max (Variables|Default|GetJauge%20Lait%20Max))
  (bind _returnvalue (/ _jauge_lait_actuel _jauge_lait_max))
  ;[0.15 0.15 0.15 0.5] Ajuster la jauge de lait sur les bombonnes du sac à dos en fonction de la quantité de lait
  (Rendering|Material|SetScalarParameterValue (Variables|Default|GetM_JaugeLait_Reference) "Percent" (select (== _returnvalue 0.0) -1.0 _returnvalue) :!class /Script/Engine.MaterialInstanceDynamic)
  (bind _outlaunchvelocity (Game|SuggestProjectileVelocityCustomArc (Transformation|GetSocketLocation "NozzleSocket") (Variables|/Game/ThirdPerson/Blueprints/BP_ThirdPersonCharacter.BP_ThirdPersonCharacter_C|GetPositionMondeDeLaMire (Variables|Default|GetReferencePawnJoueur)) 0.0 (Variables|Default|GetArc%20Projectile%20Lait)))
  (Variables|Default|SetNozzleRotation (Math|Conversions|RotationFromXVector _outlaunchvelocity)))

(event Input|KeyboardEvents|DebugKeyM
  (params (Key :type Key%20Structure :default "None") (ActionValue :type Input%20Action%20Value%20Structure))
  ;[0.149 0 0 0.502] Debug remplir le lait au max
  (:Pressed
    (Variables|Default|SetJauge%20Lait%20Actuel (Variables|Default|GetJauge%20Lait%20Max))))

(fn AjusterJaugeLait
  (params (QuantiteLait :type Float%20%28double-precision%29))
  (Variables|Default|SetJauge%20Lait%20Actuel (Math|Float|Clamp(Float) (+ QuantiteLait (Variables|Default|GetJauge%20Lait%20Actuel)) 0.0 (Variables|Default|GetJauge%20Lait%20Max)))
  (return))

(fn UtiliserLait
  (if (> (Variables|Default|GetJauge%20Lait%20Actuel) 0.0)
    (bind _result (Math|Float|NegateFloat (* (Utilities|Time|GetWorldDeltaSeconds) (Variables|Default|GetLait%20Per%20Second)))
      (:%20%20
        (CallFunction|AjusterJaugeLait _result)
        (return false)))
    (else
      (return true))))

(fn RemplirLait
  (if (== (Variables|Default|GetJauge%20Lait%20Actuel) (Variables|Default|GetJauge%20Lait%20Max))
    (return true)
    (else
      (CallFunction|AjusterJaugeLait (* (Utilities|Time|GetWorldDeltaSeconds) (* (Variables|Default|GetLait%20Per%20Second) 4.0)))
      (return false))))