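; Base-style interactive object that offers the player an interaction while they overlap it, with Interact and EndInteract events left empty.
; Overlap stores the third-person character, shows the ToucheInteraction key prompt and adds the IMC_Interagir Enhanced Input mapping context; leaving reverses this.
; When OrientText is set, Tick turns the Scene component toward the player's follow camera, noted as keeping remaining-ammo text readable.
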(event Custom|Interact
  (params (ReferenceToCharacter :type BP%20Third%20Person%20Character%20Object%20Reference)))

(event Custom|EndInteract)

(event EventBeginPlay
  (Rendering|SetVisibility (Variables|Default|GetToucheInteraction) false true))

(event Collision|EventActorBeginOverlap
  (params (OtherActor :type Actor%20Object%20Reference))
  (bind _asbp_third_person_character (Utilities|Casting|CastToBP_ThirdPersonCharacter OtherActor))
  (bind _output_get (Variables|Default|SetReferenceToPlayerCharacter _asbp_third_person_character))
  (CallFunction|AjouterActionInteragir _output_get)
  (Rendering|SetVisibility (Variables|Default|GetToucheInteraction) true true))

(event Collision|EventActorEndOverlap
  (params (OtherActor :type Actor%20Object%20Reference))
  (bind _asbp_third_person_character (Utilities|Casting|CastToBP_ThirdPersonCharacter OtherActor))
  (CallFunction|RetirerActionInteragir _asbp_third_person_character)
  (Variables|Default|SetReferenceToPlayerCharacter 0)
  (Rendering|SetVisibility (Variables|Default|GetToucheInteraction) false true))

(event EventTick
  (params (DeltaSeconds :type Float%20%28single-precision%29))
  (bind _scene (Variables|Default|GetScene))
  ;[0.15 0.15 0.15 0.5] Oriente le texte affichant le nombre de munition restante vers la caméra du joueur
  (if (Variables|Default|GetOrientText?)
    (bind _asbp_third_person_character (Utilities|Casting|CastToBP_ThirdPersonCharacter (Game|Player|GetPlayerPawn 0)))
    (Transformation|SetWorldRotation _scene (Math|Rotator|FindLookatRotation (Transformation|GetWorldLocation _scene) (Transformation|GetWorldLocation (Variables|/Game/ThirdPerson/Blueprints/BP_ThirdPersonCharacter.BP_ThirdPersonCharacter_C|GetFollowCamera _asbp_third_person_character))) false false)))

(fn ConstructionScript)

(fn AjouterActionInteragir
  (params (ReferenceToPlayer :type BP%20Third%20Person%20Character%20Object%20Reference))
  (bind _asplayer_controller (Utilities|Casting|CastToPlayerController (Pawn|GetController ReferenceToPlayer)))
  (Input|AddMappingContext (PlayerController|LocalPlayerSubsystems|GetEnhancedInputLocalPlayerSubsystem _asplayer_controller) "/Game/ThirdPerson/Input/IMC_Interagir.IMC_Interagir" 0 "(bIgnoreAllPressedKeysUntilRelease=True,bForceImmediately=False,bNotifyUserSettings=False)"))

(fn RetirerActionInteragir
  (params (ReferenceToPlayer :type BP%20Third%20Person%20Character%20Object%20Reference))
  (bind _asplayer_controller (Utilities|Casting|CastToPlayerController (Pawn|GetController ReferenceToPlayer)))
  (Input|RemoveMappingContext (PlayerController|LocalPlayerSubsystems|GetEnhancedInputLocalPlayerSubsystem _asplayer_controller) "/Game/ThirdPerson/Input/IMC_Interagir.IMC_Interagir" "(bIgnoreAllPressedKeysUntilRelease=True,bForceImmediately=False,bNotifyUserSettings=False)"))