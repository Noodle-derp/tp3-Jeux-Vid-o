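; Rifle component for the third-person character that handles shooting and ammunition.
; The shoot input fires only when the owner is aiming, not falling and has ammo, spawning a projectile from the nozzle socket toward the crosshair's world position.
; A DoOnce reset after a delay limits fire rate; the line trace result goes unused.
; A refill function returns excess rounds, alongside a full-ammo check and debug refill key.
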(event Custom|ResetTir
  (bind _returnvalue (Transformation|GetSocketLocation "nozzle"))
  (bind _referencetoowner (Variables|Default|GetReferenceToOwner))
  (bind _positionmondedelamire (Variables|/Game/ThirdPerson/Blueprints/BP_ThirdPersonCharacter.BP_ThirdPersonCharacter_C|GetPositionMondeDeLaMire _referencetoowner))
  ;[0.15 0.15 0.15 0.5 64] Shooting
  (Utilities|FlowControl|DoOnce false) ; enters at Reset
)

(event Input|EnhancedActionEvents|EnhancedInputActionIA_Shoot
  (params (ActionValue :type Boolean) (ElapsedSeconds :type Float%20%28double-precision%29) (TriggeredSeconds :type Float%20%28double-precision%29) (InputAction :type Input%20Action%20Object%20Reference :default "/Game/ThirdPerson/Input/Actions/IA_Shoot.IA_Shoot"))
  (bind _returnvalue (Transformation|GetSocketLocation "nozzle"))
  (bind _referencetoowner (Variables|Default|GetReferenceToOwner))
  (bind _referencetoowner_2 (Variables|Default|GetReferenceToOwner))
  (bind _positionmondedelamire (Variables|/Game/ThirdPerson/Blueprints/BP_ThirdPersonCharacter.BP_ThirdPersonCharacter_C|GetPositionMondeDeLaMire _referencetoowner))
  ;[0.15 0.15 0.15 0.5 64] Shooting
  (if (Math|Boolean|ANDBoolean (not (AI|Components|NavMovement|IsFalling (Variables|/Script/Engine.Character|GetCharacterMovement _referencetoowner_2))) (> (Variables|Default|GetMunitions) 0) (Variables|/Game/ThirdPerson/Blueprints/BP_ThirdPersonCharacter.BP_ThirdPersonCharacter_C|GetIsAiming _referencetoowner_2))
    (Utilities|FlowControl|DoOnce false
      (:Completed
        (Collision|LineTraceByChannel _returnvalue _positionmondedelamire "TraceTypeQuery1" false 0 "None" true "(R=1.000000,G=0.000000,B=0.000000,A=1.000000)" "(R=0.000000,G=1.000000,B=0.000000,A=1.000000)" 0.1)
        (Game|SpawnActorfromClass "/Game/Blueprint/Projectiles/BP_Projectile_Gun.BP_Projectile_Gun_C" (Math|Transform|MakeTransform _returnvalue (Math|Rotator|FindLookatRotation _returnvalue _positionmondedelamire) "1.000000,1.000000,1.000000") "Undefined" "MultiplyWithRoot" 0 (Variables|Default|GetReferenceToOwner self))
        (Math|Integer|DecrementInt (Variables|Default|GetMunitions)
          (:%20%20
            (Utilities|FlowControl|Delay (Variables|Default|GetCadence%20Tir))
            (CallFunction|ResetTir)))))))

(event EventBeginPlay
  (bind _asbp_third_person_character (Utilities|Casting|CastToBP_ThirdPersonCharacter (Components|GetOwner)))
  (Variables|Default|SetReferenceToOwner _asbp_third_person_character))

(event EventTick
  (params (DeltaSeconds :type Float%20%28single-precision%29)))

(event Input|KeyboardEvents|DebugKeyM
  (params (Key :type Key%20Structure :default "None") (ActionValue :type Input%20Action%20Value%20Structure))
  ;[0.15 0.15 0.15 0.5] Débogue ajouter des munitions
  (:Pressed
    (Variables|Default|SetMunitions (Variables|Default|GetMunitionsMax))))

(fn MunitionsPleines?
  (return (== (Variables|Default|GetMunitions) (Variables|Default|GetMunitionsMax))))

(fn RemplirMunitions
  (params (QuantiteMunitions :type Integer))
  (LocalVariables|SetExcedantMunitions (Math|Integer|Clamp(Integer) (- QuantiteMunitions (- (Variables|Default|GetMunitionsMax) (Variables|Default|GetMunitions))) 0 QuantiteMunitions))
  ;[0.15 0.15 0.15 0.5] Rempli les munitions
  (Variables|Default|SetMunitions (Math|Integer|Clamp(Integer) (+ QuantiteMunitions (Variables|Default|GetMunitions)) 0 (Variables|Default|GetMunitionsMax)))
  (return (LocalVariables|GetExcedantMunitions)))