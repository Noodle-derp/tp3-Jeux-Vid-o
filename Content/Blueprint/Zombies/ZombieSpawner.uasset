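; Zombie spawner actor that keeps one zombie alive in the world, spawning a replacement whenever its current one is no longer valid.
; Tick polls the stored zombie reference and calls SpawnZombie when it is invalid, storing the result.
; SpawnZombie picks a random class from ZombieClassReference, spawns it at the Capsule's world transform, and makes the new zombie's Sphere component visible in game.
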(event EventBeginPlay)

(event Collision|EventActorBeginOverlap
  (params (OtherActor :type Actor%20Object%20Reference)))

(event EventTick
  (params (DeltaSeconds :type Float%20%28single-precision%29))
  (Utilities|IsValid (Variables|Default|GetZombie%20Reference)
    (:Is%20Not%20Valid
      (bind _zombiereference (CallFunction|SpawnZombie))
      (Variables|Default|SetZombie%20Reference _zombiereference))))

(fn ConstructionScript)

(fn SpawnZombie
  (bind _returnvalue (Game|SpawnActorfromClass (.OutItem (Utilities|Array|Random (Variables|Default|GetZombieClassReference))) (Transformation|GetWorldTransform (Variables|Default|GetCapsule)) "Undefined" "MultiplyWithRoot" 0 0))
  (Development|SetHiddeninGame (Variables|/Game/Blueprint/Zombies/BP_Zombie_Parent.BP_Zombie_Parent_C|GetSphere _returnvalue) false false)
  (Rendering|SetVisibility (Variables|/Game/Blueprint/Zombies/BP_Zombie_Parent.BP_Zombie_Parent_C|GetSphere _returnvalue) true false)
  (return _returnvalue))