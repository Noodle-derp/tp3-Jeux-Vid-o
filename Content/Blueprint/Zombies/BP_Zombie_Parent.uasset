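; Base zombie enemy character that chases, attacks and reacts to gunfire, with randomized looping-style ambient voice and walk/run speed switches.
; Attack plays a montage once at a time, while a right-hand sphere trace damages the player once per swing.
; Bumping the player reports a touch event to AI perception.
; Point damage spawns goo particles and physics-launched goo spawners, adding headshot effects; health component death spawns goo and destroys it.
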(event OnDeath(AC_JaugeVie)
  (CallFunction|SpawnGoo (Transformation|GetWorldLocation (Variables|Character|GetMesh)) "0, 0, 0" "None" 2e+02)
  (Actor|DestroyActor))

(event OnComponentHit(CapsuleComponent)
  (params (HitComponent :type Primitive%20Component%20Object%20Reference) (OtherActor :type Actor%20Object%20Reference) (OtherComp :type Primitive%20Component%20Object%20Reference) (NormalImpulse :type Vector :default "0, 0, 0") (Hit :type Hit%20Result%20Structure%20%28by%20ref%29))
  (bind _asbp_third_person_character (Utilities|Casting|CastToBP_ThirdPersonCharacter OtherActor))
  (Class|AISenseTouch|ReportTouchEvent self _asbp_third_person_character "0, 0, 0"))

(event Custom|Attaque
  (Utilities|FlowControl|DoOnce false :!label _label
    (:Completed
      (Animation|Montage|PlayMontage (Variables|Character|GetMesh) "/Game/Animations/Zombie/Zombie_Attack_01_Montage.Zombie_Attack_01_Montage" 1.0 0.2
        (:OnCompleted
          (Variables|Default|SetHitPlayer false)
          (goto _label Reset))))))

(event EventBeginPlay
  (bind _returnvalue (Audio|SpawnSoundAttached (.OutItem (Utilities|Array|Random (Utilities|Array|MakeArray "/Game/Audio/SFX/Zombie/Zombie_Running.Zombie_Running" "/Game/Audio/SFX/Zombie/Zombie_Idle.Zombie_Idle"))) (Variables|Character|GetMesh) "Head" "0, 0, 0" "0, 0, 0" "KeepRelativeOffset" true 1.0 (Math|Random|RandomFloatinRange 0.7 1.3) (Math|Random|RandomFloatinRange 0.0 5.0) "/Game/Audio/SFX/Zombie/SA_Zombie.SA_Zombie" 0))
  (Variables|Default|SetZombieBaseSound _returnvalue))

(event Collision|EventActorBeginOverlap
  (params (OtherActor :type Actor%20Object%20Reference)))

(event EventTick
  (params (DeltaSeconds :type Float%20%28single-precision%29)))

(event Game|Damage|EventPointDamage
  (params (Damage :type Float%20%28single-precision%29) (DamageType :type Damage%20Type%20Object%20Reference) (HitLocation :type Vector :default "0, 0, 0") (HitNormal :type Vector :default "0, 0, 0") (HitComponent :type Primitive%20Component%20Object%20Reference) (BoneName :type Name :default "None") (ShotFromDirection :type Vector :default "0, 0, 0") (InstigatedBy :type Controller%20Object%20Reference) (DamageCauser :type Actor%20Object%20Reference) (HitInfo :type Hit%20Result%20Structure%20%28by%20ref%29))
  (bind _mesh (Variables|Character|GetMesh))
  (bind _returnvalue (Transformation|GetSocketLocation _mesh BoneName))
  ;[0.15 0.15 0.15 0.5] FX et SFX du dommage causé par l'arme à feu
  ;;[0.15 0.15 0.15 0.5] Spawn une flaque de Goo
  (CallFunction|SpawnGoo HitLocation HitNormal BoneName 2e+02)
  (Audio|PlaySoundatLocation "/Game/Audio/SFX/GunHit.GunHit" HitLocation "0, 0, 0" 1.0 (Math|Random|RandomFloatinRange 0.9 1.1) 0.0 "/Game/Audio/SFX/Zombie/SA_Zombie.SA_Zombie" 0 0 0)
  (if (== BoneName "Head")
    (Niagara|SpawnSystemAttached "/Game/FX/NS_GooSplash_Headshot.NS_GooSplash_Headshot" _mesh BoneName _returnvalue "0, 0, 0" "KeepWorldPosition" true)
    (Audio|PlaySoundatLocation "/Game/Audio/SFX/StabJuicy.StabJuicy" _returnvalue "0, 0, 0" 1.0 (Math|Random|RandomFloatinRange 0.9 1.1) 0.1 "/Game/Audio/SFX/Zombie/SA_Zombie.SA_Zombie" 0 0 0)))

(fn ConstructionScript)

(fn SetRun
  (Variables|/Script/Engine.CharacterMovementComponent|SetMaxWalkSpeed (Variables|Character|GetCharacterMovement) (Variables|Default|GetVitesseMax)))

(fn SetWalk
  (Variables|/Script/Engine.CharacterMovementComponent|SetMaxWalkSpeed (Variables|Character|GetCharacterMovement) 1.5e+02))

(fn HitDetection
  (bind _self self)
  (bind _mesh (Variables|Character|GetMesh))
  (bind _returnvalue (Transformation|GetSocketLocation _mesh "RightHandAttack"))
  (bind _outhit (Collision|SphereTraceForObjects _returnvalue _returnvalue 4e+01 (Utilities|Array|MakeArray "ObjectTypeQuery3") false 0 "None" true "(R=1.000000,G=0.000000,B=0.000000,A=1.000000)" "(R=0.000000,G=1.000000,B=0.000000,A=1.000000)" 1.0))
  (if (not (Variables|Default|GetHitPlayer))
    (bind _asbp_third_person_character (Utilities|Casting|CastToBP_ThirdPersonCharacter (.HitActor (Collision|BreakHitResult _outhit))))
    (Game|Damage|ApplyDamage _asbp_third_person_character 1e+01 (Pawn|GetController _self) _self)
    (Variables|Default|SetHitPlayer true)))

(fn SpawnGoo
  (params (Location :type Vector) (Direction :type Vector) (BoneName :type Name) (Vitesse :type Float%20%28double-precision%29))
  ;[0.15 0.15 0.15 0.5] Spawn le systeme de particule
  (Niagara|SpawnSystemAttached "/Game/FX/NS_GooSplash.NS_GooSplash" (Variables|Character|GetMesh) BoneName Location (Math|Rotator|MakeRotfromX Direction) "KeepWorldPosition" true)
  (bind _returnvalue (Game|SpawnActorfromClass "/Game/Blueprint/Goo/BP_Goospawner.BP_GooSpawner_C" (Math|Transform|MakeTransform Location (Math|Rotator|MakeRotfromX Direction) "1.000000,1.000000,1.000000") "Undefined" "MultiplyWithRoot" 0 0))
  (Physics|AddImpulse (Variables|/Game/Blueprint/Goo/BP_Goospawner.BP_GooSpawner_C|GetSphere _returnvalue) (* (Transformation|GetActorForwardVector _returnvalue) Vitesse) "None" false))