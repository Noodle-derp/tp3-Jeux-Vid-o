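; Behavior tree task that picks a random navigable patrol point for a zombie.
; It searches inside the zombie's patrol zone sphere, or around the zombie itself when no zone is set.
; It retries points too close to the pawn, accepting one anyway after a capped number of attempts.
; It then writes the location and a random wait time to the blackboard and finishes successfully.
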(event EventReceiveExecuteAI
  (params (OwnerController :type AI%20Controller%20Object%20Reference) (ControlledPawn :type Pawn%20Object%20Reference))
  (bind _asbp_zombie_parent (Utilities|Casting|CastToBP_Zombie_Parent ControlledPawn))
  (Utilities|IsValid (Variables|/Game/Blueprint/Zombies/BP_Zombie_Parent.BP_Zombie_Parent_C|GetPatrouilleZone _asbp_zombie_parent)
    (:Is%20Valid
      (Variables|Default|SetOrigin (Transformation|GetActorLocation (Variables|/Game/Blueprint/Zombies/BP_Zombie_Parent.BP_Zombie_Parent_C|GetPatrouilleZone _asbp_zombie_parent)))
      (Variables|Default|SetRadius (Components|Sphere|GetScaledSphereRadius (Variables|/Game/ElementsJeu/Zombies/BP_ZonePatrouille.BP_ZonePatrouille_C|GetSphere (Variables|/Game/Blueprint/Zombies/BP_Zombie_Parent.BP_Zombie_Parent_C|GetPatrouilleZone _asbp_zombie_parent)))))
    (:Is%20Not%20Valid
      (Variables|Default|SetOrigin (Transformation|GetActorLocation _asbp_zombie_parent))
      (Variables|Default|SetRadius 7.5e+02)))
  (bind _randomlocation (Class|NavigationSystemV1|GetRandomLocationinNavigableRadius (Variables|Default|GetOrigin) (Variables|Default|GetRadius) 0 0 :!label _label))
  (Variables|Default|SetRandom%20Location _randomlocation)
  ;[0.15 0.15 0.15 0.5] Après un certain nombre d'essaie, on prend simplement la valeur actuel même si elle est très près
  (if (> (Math|Vector|Distance(Vector) (Transformation|GetActorLocation _asbp_zombie_parent) _randomlocation) 2e+02)
    _
    (elif (> (Variables|Default|GetAttemptAtFindingPoint) 20)
      _
      (else
        (Math|Integer|IncrementInt (Variables|Default|GetAttemptAtFindingPoint)
          (:%20%20
            (goto _label))))))
  (AI|BehaviorTree|SetBlackboardValueasVector (Variables|Default|GetPatrolLocation) (Variables|Default|GetRandom%20Location))
  (Class|BTFunctionLibrary|SetBlackboardValueasFloat (Variables|Default|GetWaitTime) (Math|Random|RandomFloatinRange 2.0 5.0))
  (AI|BehaviorTree|FinishExecute true))