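; Function library for mesh generation that fills a spline's area with a staggered equilateral-triangle grid of surface-projected points.
; MakeGridPoint sizes the grid from sampled spline extents, then line-traces each point vertically against WorldStatic, skipping misses.
; A tangent cross product and closest-point distance classify points as outside, edge or interior, snapping nearby outside points onto the spline.
; It returns positions and classification codes; a separate helper selects the larger absolute float.
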(fn MakeGridPoint
  (params (Spline :type Spline%20Component%20Object%20Reference) (TriangleSize :type Float%20%28double-precision%29) (NumSplineSample :type Integer) (MaxOffsetZ :type Float%20%28double-precision%29) (MinOffsetZ :type Float%20%28double-precision%29))
  (bind _maxtrianglesize (LocalVariables|GetMaxTriangleSize))
  (bind _maxtrianglesize_2 (LocalVariables|GetMaxTriangleSize))
  (bind _returnvalue (Math|Float|Clamp(Float) TriangleSize 2.0 _maxtrianglesize_2))
  (bind _returnvalue_2 (Math|Float|Clamp(Float) TriangleSize 2.0 _maxtrianglesize))
  (LocalVariables|SetSplineOrigin (Transformation|GetWorldLocation Spline))
  (Utilities|FlowControl|Sequence
    (:then_0
      ;[0.15 0.15 0.15 0.5] Custom Box Extent pour la spline
      (for _index (range 0 NumSplineSample)
        (LocalVariables|SetCustomBoxExtent (Math|Vector|MakeVector (Math|Float|Max(Float) (.x (LocalVariables|GetCustomBoxExtent)) (Math|Float|Absolute(Float) (.X (Math|Vector|BreakVector (Spline|GetLocationatDistanceAlongSpline Spline (* (/ (Math|Conversions|ToFloat(Integer) _index) 1e+02) (Spline|GetSplineLength Spline)) "Local"))))) (Math|Float|Max(Float) (.y (LocalVariables|GetCustomBoxExtent)) (Math|Float|Absolute(Float) (.Y (Math|Vector|BreakVector (Spline|GetLocationatDistanceAlongSpline Spline (* (/ (Math|Conversions|ToFloat(Integer) _index) 1e+02) (Spline|GetSplineLength Spline)) "Local"))))) 0.0))))
    (:then_1
      ;[0.15 0.15 0.15 0.5] Calcule le nombre de vertice en X et en Y pour générer les triangles en fonction des limites de la spline et de la taille voulu des triangles
      (LocalVariables|SetNombrePointsX (Math|Float|Ceil (+ (/ (.X (Math|Vector|BreakVector (LocalVariables|GetCustomBoxExtent))) _returnvalue_2) 1.0)))
      (LocalVariables|SetNombrePointsY (Math|Float|Ceil (+ (* (/ (/ (.Y (Math|Vector|BreakVector (LocalVariables|GetCustomBoxExtent))) _returnvalue_2) 2.0) (Math|Float|Sqrt 3.0)) 1.0)))
      (Utilities|FlowControl|Sequence
        (:then_0
          ;[0.15 0.15 0.15 0.5] Boucle sur le nombre de points X et Y pour calculer la position de chaque point
          (for _index_2 (range (* (LocalVariables|GetNombrePointsY) -1) (LocalVariables|GetNombrePointsY))
            (LocalVariables|SetIndexY _index_2)
            (for _index_3 (range (* -1 (LocalVariables|GetNombrePointsX)) (LocalVariables|GetNombrePointsX))
              (LocalVariables|SetIndexX _index_3)
              ;[0.04167 0.04167 0.04167 0.5] Calcule de la position du point courant
              (LocalVariables|SetPointLocation (Math|Vector|MakeVector (+ (.X (Math|Vector|BreakVector (LocalVariables|GetSplineOrigin))) (* (LocalVariables|GetIndexX) _returnvalue) (* (Math|Integer|%(Integer) (Math|Integer|Absolute(Integer) (LocalVariables|GetIndexY)) 2) (/ _returnvalue 2.0))) (+ (.Y (Math|Vector|BreakVector (LocalVariables|GetSplineOrigin))) (* (LocalVariables|GetIndexY) (* (/ _returnvalue 2.0) (Math|Float|Sqrt 3.0)))) (.Z (Math|Vector|BreakVector (LocalVariables|GetSplineOrigin)))))
              ;[0.15 0.15 0.15 0.5] Calcule la position en Z du point selon s'il existe une surface au dessus et en dessous de la position en Z de la spline sur laquelle poser un point
              (bind _outhit (Collision|LineTraceForObjects 0 (+ (LocalVariables|GetPointLocation) (Math|Vector|MakeVector 0.0 0.0 MaxOffsetZ)) (+ (LocalVariables|GetPointLocation) (Math|Vector|MakeVector 0.0 0.0 MinOffsetZ)) (Utilities|Array|MakeArray "ObjectTypeQuery1") false 0 "None"))
              (if (and (.bBlockingHit (Collision|BreakHitResult _outhit)) (not (.bInitialOverlap (Collision|BreakHitResult _outhit))))
                (LocalVariables|SetPointLocation (Math|Vector|MakeVector (.x (LocalVariables|GetPointLocation)) (.y (LocalVariables|GetPointLocation)) (.z (.Location (Collision|BreakHitResult _outhit)))))
                ;[0.15 0.15 0.15 0.5] Vérifie si la position du point est à l'intérieur de la spline
                (LocalVariables|SetPointSplineClosest (Spline|FindLocationClosesttoWorldLocation Spline (LocalVariables|GetPointLocation) "World"))
                (LocalVariables|SetInside? (> (.z (Math|Vector|CrossProduct (Spline|FindDirectionClosesttoWorldLocation Spline (LocalVariables|GetPointLocation) "World") (- (LocalVariables|GetPointLocation) (Spline|FindLocationClosesttoWorldLocation Spline (LocalVariables|GetPointLocation) "World")))) 0.0))
                (LocalVariables|SetEdge? (< (Math|Vector|VectorLength (- (LocalVariables|GetPointLocation) (Spline|FindLocationClosesttoWorldLocation Spline (LocalVariables|GetPointLocation) "World"))) TriangleSize))
                ;[0.15 0.15 0.15 0.5] Enregistre la position et les informations du point courant dans le tableau
                (Utilities|Array|SetArrayElem (LocalVariables|GetPointsTableau) (LocalVariables|GetPointIndex) (select (and (LocalVariables|GetEdge?) (not (LocalVariables|GetInside?))) (LocalVariables|GetPointSplineClosest) (LocalVariables|GetPointLocation)) true)
                (Utilities|Array|SetArrayElem (LocalVariables|GetIndexTableau) (LocalVariables|GetPointIndex) (Math|Integer|SelectInt (Math|Integer|SelectInt 0 1 (LocalVariables|GetEdge?)) -1 (LocalVariables|GetInside?)) true)
                (Math|Integer|IncrementInt (LocalVariables|GetPointIndex))))))
        (:then_1
          (return (LocalVariables|GetPointsTableau) (LocalVariables|GetIndexTableau)))))))

(fn SelectGreaterAbsFloat
  (params (A :type Float%20%28double-precision%29) (B :type Float%20%28double-precision%29))
  (bind _returnvalue (Math|Float|Absolute(Float) A))
  (bind _returnvalue_2 (Math|Float|Absolute(Float) B))
  (return (Math|Float|SelectFloat _returnvalue _returnvalue_2 (>= _returnvalue _returnvalue_2))))