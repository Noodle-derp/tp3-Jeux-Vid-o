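; Health gauge component that tracks its owner's health, starting at max, and exposes percentage and full-health queries.
; Owner damage events and a headshot bonus on the "Head" bone feed clamped health changes, with OnDeath called when damage leaves zero.
; Goo actors register in a list, pruned on Tick or when cleaned.
; While any remain, Tick drains health, or heals at half rate if goo-immune.
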(event Custom|OnTakeAnyDamage_Event
  (params (DamagedActor :type Actor%20Object%20Reference) (Damage :type Float%20%28single-precision%29) (DamageType :type Damage%20Type%20Object%20Reference) (InstigatedBy :type Controller%20Object%20Reference) (DamageCauser :type Actor%20Object%20Reference))
  (CallFunction|AppliquerDommage Damage))

(event Custom|AjouterGooQuiOverlap
  (params (GooReference :type BP%20Goo%20Object%20Reference))
  (if (not (Utilities|Array|ContainsItem (Variables|Default|GetGooOverlappingList) GooReference))
    (Utilities|Array|AddUnique (Variables|Default|GetGooOverlappingList) GooReference)
    (EventDispatchers|AssignCleaned GooReference (delegate Custom|Cleaned_Event))))

(event Custom|Cleaned_Event
  (params (GooReference :type BP%20Goo%20Object%20Reference))
  (CallFunction|RetirerGooQuiOverlap GooReference))

(event Custom|OnTakePointDamage_Event
  (params (DamagedActor :type Actor%20Object%20Reference) (Damage :type Float%20%28single-precision%29) (InstigatedBy :type Controller%20Object%20Reference) (HitLocation :type Vector) (FHitComponent :type Primitive%20Component%20Object%20Reference) (BoneName :type Name) (ShotFromDirection :type Vector) (DamageType :type Damage%20Type%20Object%20Reference) (DamageCauser :type Actor%20Object%20Reference))
  ;[0.15 0.15 0.15 0.5] Un tir dans la tête fait tu dégât additionnel!
  (if (== BoneName "Head")
    (CallFunction|AppliquerDommage 2e+01)))

(event EventBeginPlay
  (CallFunction|AjusterVie (Variables|Default|GetVieMax))
  (EventDispatchers|AssignOnTakeAnyDamage (Components|GetOwner) (delegate Custom|OnTakeAnyDamage_Event))
  (EventDispatchers|AssignOnTakePointDamage (Components|GetOwner) (delegate Custom|OnTakePointDamage_Event)))

(event EventTick
  (params (DeltaSeconds :type Float%20%28single-precision%29))
  (bind _returnvalue (Utilities|Time|GetWorldDeltaSeconds))
  (bind _returnvalue_2 (* _returnvalue 1e+01))
  ;[0 1 0 0.5] Goo dégâts
  ;;[0.15 0.15 0.15 0.5] On vérifie si les "goo" dans la liste overlap toujours l'objet sur lequel la jauge se trouve. Si ce n'est pas le cas, on retire le goo de la liste.
  (for _array_element (Variables|Default|GetGooOverlappingList)
    (Utilities|IsValid _array_element
      (:Is%20Valid
        (bind _overlapping (Default|ValiderOverlap _array_element (Components|GetOwner)))
        (if (not _overlapping)
          (CallFunction|RetirerGooQuiOverlap _array_element)))))
  ;;[0.15 0.15 0.15 0.5] Applique des dommages
  (if (not (Utilities|Array|IsEmpty (Variables|Default|GetGooOverlappingList)))
    (if (Variables|Default|GetImmuniserGoo?)
      ;[0 1 0 0.5] Redonne des points de vie si immunisé au goo
      (CallFunction|AppliquerGuerison (/ _returnvalue_2 2.0))
      (else
        (CallFunction|AppliquerDommage _returnvalue_2)))))

(fn AppliquerGuerison
  (params (PointsDeVie :type Float%20%28double-precision%29))
  (CallFunction|AjusterVie PointsDeVie)
  (return))

(fn AppliquerDommage
  (params (PointsDeVie :type Float%20%28double-precision%29))
  (bind _result (Math|Float|NegateFloat PointsDeVie)
    (:%20%20
      (CallFunction|AjusterVie _result)
      (if (== (Variables|Default|GetVieActuel) 0.0)
        (Default|CallOnDeath)
        (return)
        (else
          (return))))))

(fn AugmenterVieMax)

(fn AjusterVie
  (params (PointsDeVie :type Float%20%28double-precision%29))
  ;[0.15 0.15 0.15 0.5] Ajuste les points de vie en s'assurant de rester entre les valeurs possible
  (Variables|Default|SetVieActuel (Math|Float|Clamp(Float) (+ PointsDeVie (Variables|Default|GetVieActuel)) 0.0 (Variables|Default|GetVieMax)))
  (return))

(fn GetViePourcentage
  (return (/ (Variables|Default|GetVieActuel) (Variables|Default|GetVieMax))))

(fn RetirerGooQuiOverlap
  (params (GooOverlapReference :type BP%20Goo%20Object%20Reference))
  (Utilities|Array|RemoveItem (Variables|Default|GetGooOverlappingList) GooOverlapReference))

(fn ViePleine?
  (return (== (Variables|Default|GetVieActuel) (Variables|Default|GetVieMax))))