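; AC_GooSpawner is a scene component that makes a zombie spawn goo as it moves.
; It stores its world location on BeginPlay and checks every tick whether it has moved more than a set distance from it.
; When it has, it updates the stored location and calls SpawnGoo on its BP_Zombie_Parent owner, aimed straight down with the Hips bone and zero speed.
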(event EventBeginPlay
  (Variables|Default|SetCurrentLocation (Transformation|GetWorldLocation)))

(event EventTick
  (params (DeltaSeconds :type Float%20%28single-precision%29))
  (if (> (Math|Vector|Distance(Vector) (Transformation|GetWorldLocation) (Variables|Default|GetCurrentLocation)) 1e+02)
    (Variables|Default|SetCurrentLocation (Transformation|GetWorldLocation))
    (bind _asbp_zombie_parent (Utilities|Casting|CastToBP_Zombie_Parent (Components|GetOwner)))
    (Default|SpawnGoo _asbp_zombie_parent (Transformation|GetWorldLocation) "0.000000,0.000000,-1.000000" "Hips" 0.0)))