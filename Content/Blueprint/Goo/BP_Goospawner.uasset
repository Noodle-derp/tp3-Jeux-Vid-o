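; BP_Goospawner is an actor that leaves a goo puddle when its sphere hits something, avoiding placement on existing goo.
; On hit, a 25-unit multi sphere trace on the Visibility channel clears the SpawnGoo flag if it finds a BP_Goo actor.
; If the flag remains set, it spawns BP_Goo_Puddle at its own location.
; It then destroys itself.
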(event OnComponentHit(Sphere)
  (params (HitComponent :type Primitive%20Component%20Object%20Reference) (OtherActor :type Actor%20Object%20Reference) (OtherComp :type Primitive%20Component%20Object%20Reference) (NormalImpulse :type Vector :default "0, 0, 0") (Hit :type Hit%20Result%20Structure%20%28by%20ref%29))
  (bind _sphere (Variables|Default|GetSphere))
  (bind _returnvalue (Transformation|GetWorldLocation _sphere))
  (bind _outhits (Collision|MultiSphereTraceByChannel _returnvalue _returnvalue 25.0 "TraceTypeQuery1" false 0 "None"))
  (for _array_element _outhits
    (Utilities|Casting|CastToBP_Goo (.HitActor (Collision|BreakHitResult _array_element)))
    (Variables|Default|SetSpawn%20Goo? false))
  (if (Variables|Default|GetSpawn%20Goo?)
    (Game|SpawnActorfromClass "/Game/ElementsJeu/Goo/BP_Goo_Puddle.BP_Goo_Puddle_C" (Math|Transform|MakeTransform (.location (Transformation|GetActorTransform)) "0, 0, 0" "1.000000,1.000000,1.000000") "AlwaysSpawn" "MultiplyWithRoot" 0 0))
  (Actor|DestroyActor))

(event EventBeginPlay)

(event Collision|EventActorBeginOverlap
  (params (OtherActor :type Actor%20Object%20Reference)))

(event EventTick
  (params (DeltaSeconds :type Float%20%28single-precision%29)))

(fn ConstructionScript)