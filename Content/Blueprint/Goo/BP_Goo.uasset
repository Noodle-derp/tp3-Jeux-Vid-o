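; Cleanable goo patch built from instanced static mesh instances, which registers itself with the AC_JaugeVie life gauge component of overlapping actors.
; CleanGoo removes instances within a sphere and checks the remainder against the initial count.
; Once the clean percentage is reached, it disables collision, shrinks the remaining instances over a timeline, then destroys itself.
; ValiderOverlap confirms actual contact using an instance box query refined by per-instance sphere traces.
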(event Custom|OnCleaned
  (bind _goo_instancedstaticmesh (Variables|Default|GetGoo_InstancedStaticMesh))
  (Default|CallCleaned self)
  (Collision|SetCollisionEnabled (Variables|Default|GetGoo_InstancedStaticMesh) "NoCollision")
  ;[0.15 0.15 0.15 0.5] Lorsque la zone des Goo est assez nettoyé, on réduit progressivement l'échelle du goo restant avant de le faire complètement disparaître
  (bind _scale (Timeline|Timeline_CleanAllGoo Play)
    (:Update
      (for _index (range 0 (Components|InstancedStaticMesh|GetInstanceCount _goo_instancedstaticmesh))
        (Components|InstancedStaticMesh|UpdateInstanceTransform _goo_instancedstaticmesh _index (Math|Transform|MakeTransform (.location (.OutInstanceTransform (Components|InstancedStaticMesh|GetInstanceTransform _goo_instancedstaticmesh _index false))) (.rotation (.OutInstanceTransform (Components|InstancedStaticMesh|GetInstanceTransform _goo_instancedstaticmesh _index false))) (* (.scale (.OutInstanceTransform (Components|InstancedStaticMesh|GetInstanceTransform _goo_instancedstaticmesh _index false))) (Math|Conversions|ToVector(Float) _scale))) false false false)))
    (:Finished
      (Actor|DestroyActor))))

(event EventBeginPlay
  (Utilities|FlowControl|Delay 0.2)
  (CallFunction|SetGooInstanceCount))

(event Collision|EventActorBeginOverlap
  (params (OtherActor :type Actor%20Object%20Reference))
  (bind _returnvalue (Actor|GetComponentbyClass OtherActor "/Game/Blueprint/AC_JaugeVie.AC_JaugeVie_C"))
  (Utilities|IsValid _returnvalue
    (:Is%20Valid
      (Default|AjouterGooQuiOverlap _returnvalue self))))

(fn ConstructionScript
  (CallFunction|GenerateGoo)
  (CallFunction|SetGooInstanceCount)
  (Components|Timeline|SetPlayRate (Variables|Default|GetTimeline_CleanAllGoo) (/ 1.0 (Variables|Default|GetCleanupTime))))

(fn GenerateGoo
  (Components|InstancedStaticMesh|AddInstance (Variables|Default|GetGoo_InstancedStaticMesh) (Math|Transform|MakeTransform "0, 0, 0" "0, 0, 0" "1.000000,1.000000,1.000000") false))

(fn CleanGoo
  (params (Position :type Vector) (Rayon :type Float%20%28double-precision%29))
  (for _array_element (Class|InstancedStaticMeshComponent|GetInstancesOverlappingSphere (Variables|Default|GetGoo_InstancedStaticMesh) Position Rayon true)
    (Class|InstancedStaticMeshComponent|RemoveInstance (Variables|Default|GetGoo_InstancedStaticMesh) _array_element)
    (bind _cleaned_ (CallFunction|CheckifAllCleaned))
    (if _cleaned_
      (CallFunction|OnCleaned))))

(fn CheckifAllCleaned
  (return (<= (/ (Math|Conversions|ToFloat(Integer) (Components|InstancedStaticMesh|GetInstanceCount (Variables|Default|GetGoo_InstancedStaticMesh))) (Math|Conversions|ToFloat(Integer) (Variables|Default|GetGooTotalCount))) (- 1.0 (/ (Variables|Default|GetPourcentagePourConsidererPropre) 1e+02)))))

(fn SetGooInstanceCount
  (Variables|Default|SetGooTotalCount (Components|InstancedStaticMesh|GetInstanceCount (Variables|Default|GetGoo_InstancedStaticMesh))))

(fn GetGooCount
  (return (Components|InstancedStaticMesh|GetInstanceCount (Variables|Default|GetGoo_InstancedStaticMesh))))

(fn ValiderOverlap
  (params (OtherActorOverlapping :type Actor%20Object%20Reference))
  (bind (_origin _boxextent) (Collision|GetActorBounds OtherActorOverlapping true false))
  (bind _goo_instancedstaticmesh (Variables|Default|GetGoo_InstancedStaticMesh))
  (bind _returnvalue (Class|KismetMathLibrary|MakeBoxwithOrigin _origin _boxextent))
  (bind _returnvalue_2 (Class|InstancedStaticMeshComponent|GetInstancesOverlappingBox _goo_instancedstaticmesh _returnvalue true))
  (Utilities|IsValid OtherActorOverlapping
    (:Is%20Valid
      (if (Utilities|Array|IsNotEmpty _returnvalue_2)
        (for _array_element _returnvalue_2
          (bind _outhit (Collision|SphereTraceForObjects (.location (.OutInstanceTransform (Components|InstancedStaticMesh|GetInstanceTransform (Variables|Default|GetGoo_InstancedStaticMesh) _array_element true))) (.location (.OutInstanceTransform (Components|InstancedStaticMesh|GetInstanceTransform (Variables|Default|GetGoo_InstancedStaticMesh) _array_element true))) (* (.x (.scale (.OutInstanceTransform (Components|InstancedStaticMesh|GetInstanceTransform (Variables|Default|GetGoo_InstancedStaticMesh) _array_element true)))) 5e+01) (Utilities|Array|MakeArray "ObjectTypeQuery3" "ObjectTypeQuery2") false 0 "None" true "(R=1.000000,G=0.000000,B=0.000000,A=1.000000)" "(R=0.000000,G=1.000000,B=0.000000,A=1.000000)" 1.0))
          (if (== (.HitActor (Collision|BreakHitResult _outhit)) OtherActorOverlapping)
            (return true)))
        (else
          (return false))))))