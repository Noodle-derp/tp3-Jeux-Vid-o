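; Milk ("Lait") projectile that leaves a BP_Clean actor where it hits, then destroys itself.
; Tick grows the collision sphere from zero to its small final scale over about half a second.
; On hit, it spawns BP_Clean with random yaw and size, and has a one-in-three chance of playing a quiet, pitch-randomized bubble sound at that location.
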(event OnComponentHit(SphereCollision)
  (params (HitComponent :type Primitive%20Component%20Object%20Reference) (OtherActor :type Actor%20Object%20Reference) (OtherComp :type Primitive%20Component%20Object%20Reference) (NormalImpulse :type Vector :default "0, 0, 0") (Hit :type Hit%20Result%20Structure%20%28by%20ref%29))
  (Game|SpawnActorfromClass "/Game/ElementsJeu/Goo/BP_Clean.BP_Clean_C" (Math|Transform|MakeTransform (Transformation|GetActorLocation self) (Math|Rotator|MakeRotator 0.0 0.0 (Math|Random|RandomFloatinRange 0.0 3.6e+02)) (Math|Conversions|ToVector(Float) (Math|Random|RandomFloatinRange 1.0 2.0))) "Undefined" "MultiplyWithRoot" 0 0)
  (Utilities|FlowControl|Sequence
    (:then_0
      (if (== (Math|Random|RandomIntegerinRange 0 2) 1)
        (Audio|PlaySoundatLocation "/Game/Audio/SFX/Bubble_02.Bubble_02" (Transformation|GetActorLocation) "0, 0, 0" 0.25 (Math|Random|RandomFloatinRange 0.1 1.0) 0.0 "/Game/Audio/SFX/Zombie/SA_Zombie.SA_Zombie" 0 0 0)))
    (:then_1
      (Actor|DestroyActor))))

(event EventBeginPlay
  (|CallParentFunction))

(event Collision|EventActorBeginOverlap
  (params (OtherActor :type Actor%20Object%20Reference))
  (|CallParentFunction OtherActor) ; This node is disabled and will not be called.\nDrag off pins to build functionality.
)

(event EventTick
  (params (DeltaSeconds :type Float%20%28single-precision%29))
  (|CallParentFunction DeltaSeconds)
  (bind _output_get (Variables|Default|SetScale (Math|Float|Clamp(Float) (+ (* DeltaSeconds 2.0) (Variables|Default|GetScale)))))
  (Transformation|SetWorldScale3D (Variables|Default|GetSphereCollision) (Math|Conversions|ToVector(Float) (Math|Float|Lerp 0.0 0.25 _output_get))))

(fn ConstructionScript
  (|CallParentFunction))