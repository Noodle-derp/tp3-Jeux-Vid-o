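; BP_Projectile_Gun is a gun projectile that damages what it hits and reports its activity as noise and damage events.
; On BeginPlay it plays a placeholder paintball sound with randomized volume and pitch, then reports a noise event with limited range.
; When its collision sphere hits something, it applies fixed point damage, reports a damage event attributed to the instigator, and destroys itself.
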(event OnComponentHit(SphereCollision)
  (params (HitComponent :type Primitive%20Component%20Object%20Reference) (OtherActor :type Actor%20Object%20Reference) (OtherComp :type Primitive%20Component%20Object%20Reference) (NormalImpulse :type Vector :default "0, 0, 0") (Hit :type Hit%20Result%20Structure%20%28by%20ref%29))
  (Game|Damage|ApplyPointDamage OtherActor 2e+01 NormalImpulse Hit)
  (Class|AISenseDamage|ReportDamageEvent OtherActor (Variables|Default|GetInstigator) 0.0 "0, 0, 0" "0, 0, 0" "None")
  (Actor|DestroyActor))

(event EventBeginPlay
  (bind _sphere (Variables|Default|GetSphere))
  (bind _returnvalue (Transformation|GetWorldLocation _sphere))
  (|CallParentFunction)
  ;[0.15 0.15 0.15 0.5] Son placeholder
  (Audio|PlaySoundatLocation "/Game/Audio/SFX/Paintball.Paintball" _returnvalue "0, 0, 0" (Math|Random|RandomFloatinRange 1.0 2.0) (Math|Random|RandomFloatinRange 0.65 1.0) 0.0 0 0 0 0)
  (Class|AISenseHearing|ReportNoiseEvent _returnvalue 1.0 (Variables|Default|GetInstigator) 1e+03 "None"))

(event Collision|EventActorBeginOverlap
  (params (OtherActor :type Actor%20Object%20Reference))
  (|CallParentFunction OtherActor) ; This node is disabled and will not be called.\nDrag off pins to build functionality.
)

(event EventTick
  (params (DeltaSeconds :type Float%20%28single-precision%29))
  (|CallParentFunction DeltaSeconds) ; This node is disabled and will not be called.\nDrag off pins to build functionality.
)

(fn ConstructionScript
  (|CallParentFunction))