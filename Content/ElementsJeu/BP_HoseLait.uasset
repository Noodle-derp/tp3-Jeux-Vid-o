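; BP_HoseLait is an interactable pickup actor that equips the interacting character with a milk hose.
; On Interact, it adds an AC_HoseLait component to that character at runtime and attaches it to the "Backpack" socket on the character's mesh, keeping relative transforms.
; The pickup then destroys itself, and it has no other active logic.
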(event EventBeginPlay
  (|CallParentFunction) ; This node is disabled and will not be called.\nDrag off pins to build functionality.
)

(event Collision|EventActorBeginOverlap
  (params (OtherActor :type Actor%20Object%20Reference))
  (|CallParentFunction OtherActor) ; This node is disabled and will not be called.\nDrag off pins to build functionality.
)

(event EventTick
  (params (DeltaSeconds :type Float%20%28single-precision%29))
  (|CallParentFunction DeltaSeconds) ; This node is disabled and will not be called.\nDrag off pins to build functionality.
)

(event EventInteract
  (params (ReferenceToCharacter :type BP%20Third%20Person%20Character%20Object%20Reference))
  (bind _returnvalue (AddComponent|AddACHoseLait ReferenceToCharacter false))
  (Transformation|AttachComponentToComponent _returnvalue (Variables|/Script/Engine.Character|GetMesh ReferenceToCharacter) "Backpack" "KeepRelative" "KeepRelative" "KeepRelative" true)
  (Actor|DestroyActor))

(fn ConstructionScript
  (|CallParentFunction))