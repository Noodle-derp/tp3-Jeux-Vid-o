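; BP_ZoneNarration is a trigger zone that plays timed, colored narration lines when the player pawn enters it.
; It fetches the shared narration widget from GameState-TPF, registers itself as the active narration, then steps through the Narration array with a timer per line.
; A DoOnce blocks retriggering, resetting after the last line only if Repetable, when the widget is also removed.
; StopNarration clears the timer to interrupt playback.
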(event Custom|ResetOverlap
  ;[0.15 0.15 0.15 0.5] Lorsque le joueur entre dans la zone, l'index est remis à 0, puis la narration est lancé.
  (Utilities|FlowControl|DoOnce false) ; enters at Reset
)

(event Custom|StartNarration
  (bind _narration (Variables|Default|GetNarration))
  (bind _currentindex (Variables|Default|GetCurrentIndex))
  (bind _output (Utilities|Array|Get(acopy) _narration _currentindex))
  ;[0.15 0.15 0.15 0.5] On met à jour le texte, puis on établie la durée du timer (la durée où le texte reste à l'écran).
  (Default|UpdateText (Variables|Default|GetWBP_Narration) (.texte _output) (.couleur _output))
  (bind _returnvalue (Utilities|Time|SetTimerbyEvent (delegate Custom|PrepareNextLine) (.duration _output)))
  (Variables|Default|SetNarrationTimer _returnvalue))

(event Custom|StopNarration
  ;[0.15 0.15 0.15 0.5] Le timer est arrêté
  (Utilities|Time|ClearandInvalidateTimerbyHandle (Variables|Default|GetNarrationTimer)))

(event Custom|PrepareNextLine
  ;[0.15 0.15 0.15 0.5] On augmente l'index d'un, puis on vérifie si la narration est complétée.
  (Math|Integer|IncrementInt (Variables|Default|GetCurrentIndex)
    (:%20%20
      (if (< (Utilities|Array|LastIndex (Variables|Default|GetNarration)) (Variables|Default|GetCurrentIndex))
        ;[0.15 0.15 0.15 0.5] Si la narration est complétée, on retire le widget de l'écran, puis on vérifie, elle peut être relancée.
        (Widget|RemovefromParent (Variables|Default|GetWBP_Narration))
        (if (Variables|Default|GetRepetable?)
          (CallFunction|ResetOverlap))
        (else
          (CallFunction|StartNarration))))))

(event EventBeginPlay
  ;[0.15 0.15 0.15 0.5] Récupère le Widget de narration et le store dans une variable
  (Utilities|FlowControl|Delay 0.2)
  (bind _asgame_state__tpf (Utilities|Casting|CastToGameState-TPF (Game|GetGameState)))
  (Variables|Default|SetWBP_Narration (Variables|/Game/System/GameState-TPF.GameState-TPF_C|GetWBP-Narration _asgame_state__tpf)))

(event Collision|EventActorBeginOverlap
  (params (OtherActor :type Actor%20Object%20Reference))
  ;[0.15 0.15 0.15 0.5] Lorsque le joueur entre dans la zone, l'index est remis à 0, puis la narration est lancé.
  (if (== OtherActor (Game|Player|GetPlayerPawn 0))
    (Utilities|FlowControl|DoOnce false
      (:Completed
        (Default|ChangeActiveNarration (Variables|Default|GetWBP_Narration) self)
        (Variables|Default|SetCurrentIndex 0)
        (CallFunction|StartNarration)))))

(fn ConstructionScript)