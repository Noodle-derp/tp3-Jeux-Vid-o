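; Checkpoint actor that saves the player's state and respawns them at its location.
; When the player overlaps it, it becomes the GameState-TPF's active checkpoint and stores health, milk hose backpack gauge and gun ammo.
; RespawnPlayer spawns and possesses a new third-person character, restores the saved health or full health if GueritJoueur is set, and re-adds the saved backpack and gun with their amounts.
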(event Custom|RespawnPlayer
  (bind _returnvalue (Transformation|GetActorTransform))
  ;[0.15 0.15 0.15 0.5] Lorsque le joueur meurt, il est respawné, puis les valeurs gardées en mémoire lui sont réassignées.
  (bind _returnvalue_2 (Game|SpawnActorfromClass "/Game/ThirdPerson/Blueprints/BP_ThirdPersonCharacter.BP_ThirdPersonCharacter_C" (Math|Transform|MakeTransform (.location _returnvalue) (.rotation _returnvalue) "1.000000,1.000000,1.000000") "AdjustIfPossibleButAlwaysSpawn" "MultiplyWithRoot" 0 0))
  (Utilities|FlowControl|Sequence
    (:then_0
      (Variables|/Game/Blueprint/AC_JaugeVie.AC_JaugeVie_C|SetVieActuel (Variables|/Game/ThirdPerson/Blueprints/BP_ThirdPersonCharacter.BP_ThirdPersonCharacter_C|GetAC_JaugeVie _returnvalue_2) (Math|Float|SelectFloat (Variables|/Game/Blueprint/AC_JaugeVie.AC_JaugeVie_C|GetVieMax (Variables|/Game/ThirdPerson/Blueprints/BP_ThirdPersonCharacter.BP_ThirdPersonCharacter_C|GetAC_JaugeVie _returnvalue_2)) (Variables|Default|GetJoueur-Vie) (Variables|Default|GetGueritJoueur?)))
      (if (Variables|Default|GetJoueur-BackBack)
        (bind _returnvalue_3 (AddComponent|AddACHoseLait _returnvalue_2 false))
        (Transformation|AttachComponentToComponent _returnvalue_3 (Variables|/Script/Engine.Character|GetMesh _returnvalue_2) "Backpack" "KeepRelative" "KeepRelative" "KeepRelative" true)
        (Variables|/Game/Blueprint/Lait/AC_HoseLait.AC_HoseLait_C|SetJauge%20Lait%20Actuel _returnvalue_3 (Variables|Default|GetJoueur-Lait)))
      (Pawn|Possess (Game|GetPlayerController 0) _returnvalue_2))
    (:then_1
      (if (Variables|Default|GetJoueur-Fusil)
        (bind _ac_fusil (Default|AjouterFusil _returnvalue_2))
        (Utilities|IsValid _ac_fusil
          (:Is%20Valid
            (Variables|/Game/Blueprint/AC_Fusil.AC_Fusil_C|SetMunitions _ac_fusil (Variables|Default|GetJoueur-Munition))))))))

(event EventBeginPlay
  (bind _asgame_state__tpf (Utilities|Casting|CastToGameState-TPF (Game|GetGameState)))
  (Variables|Default|SetGameState-TPF _asgame_state__tpf))

(event Collision|EventActorBeginOverlap
  (params (OtherActor :type Actor%20Object%20Reference))
  ;[0.15 0.15 0.15 0.5] Lorsque le joueur entre dans la zone du checkpoint, celui-ci devient actif et garde en mémoire l'état du joueur.
  (if (== OtherActor (Game|Player|GetPlayerPawn 0))
    (Variables|/Game/System/GameState-TPF.GameState-TPF_C|SetActiveCheckpoint (Variables|Default|GetGameState-TPF) self)
    (bind _asbp_third_person_character (Utilities|Casting|CastToBP_ThirdPersonCharacter (Game|GetPlayerCharacter 0)))
    (Utilities|FlowControl|Sequence
      (:then_0
        (Variables|Default|SetJoueur-Vie (Variables|/Game/Blueprint/AC_JaugeVie.AC_JaugeVie_C|GetVieActuel (Variables|/Game/ThirdPerson/Blueprints/BP_ThirdPersonCharacter.BP_ThirdPersonCharacter_C|GetAC_JaugeVie _asbp_third_person_character)))
        (Utilities|IsValid (Utilities|Array|Get(acopy) (Actor|GetComponentsByClass _asbp_third_person_character "/Game/Blueprint/Lait/AC_HoseLait.AC_HoseLait_C"))
          (:Is%20Valid
            (Variables|Default|SetJoueur-BackBack true)
            (Variables|Default|SetJoueur-Lait (Variables|/Game/Blueprint/Lait/AC_HoseLait.AC_HoseLait_C|GetJauge%20Lait%20Actuel (Utilities|Array|Get(acopy) (Actor|GetComponentsByClass _asbp_third_person_character "/Game/Blueprint/Lait/AC_HoseLait.AC_HoseLait_C")))))))
      (:then_1
        (Utilities|IsValid (Actor|GetComponentbyClass _asbp_third_person_character "/Game/Blueprint/AC_Fusil.AC_Fusil_C")
          (:Is%20Valid
            (Variables|Default|SetJoueur-Fusil true)
            (Variables|Default|SetJoueur-Munition (Variables|/Game/Blueprint/AC_Fusil.AC_Fusil_C|GetMunitions (Actor|GetComponentbyClass _asbp_third_person_character "/Game/Blueprint/AC_Fusil.AC_Fusil_C")))))))))

(fn ConstructionScript)