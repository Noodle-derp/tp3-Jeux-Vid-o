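; BP_Goo_Puddle is a goo element that forms a puddle from randomly scattered blobs.
; The construction script calls GenerateGoo, which runs the parent version, then adds a fixed number of instances to GooInstancedStaticMesh.
; Each blob gets a random X/Y offset within plus or minus Radius, so the spread is square, and a random uniform scale.
; The event graph holds no active logic.
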(event EventBeginPlay)

(event Collision|EventActorBeginOverlap
  (params (OtherActor :type Actor%20Object%20Reference)))

(event EventTick
  (params (DeltaSeconds :type Float%20%28single-precision%29)))

(fn ConstructionScript
  (CallFunction|GenerateGoo))

(fn GenerateGoo
  (bind _radius (Variables|Default|GetRadius))
  (bind _returnvalue (* _radius -1.0))
  (|CallParentFunction)
  ;[0.15 0.15 0.15 0.5] Spawn quelques blob de goo de façon randomisé dans un rayon
  (for _index (range 0 10)
    (Components|InstancedStaticMesh|AddInstance (Variables|Default|GetGoo_InstancedStaticMesh) (Math|Transform|MakeTransform (Math|Vector|MakeVector (Math|Random|RandomFloatinRange _returnvalue _radius) (Math|Random|RandomFloatinRange _returnvalue _radius) 0.0) "0, 0, 0" (Math|Conversions|ToVector(Float) (Math|Random|RandomFloatinRange 0.75 1.25))) false)))