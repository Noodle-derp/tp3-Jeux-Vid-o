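; BP_Goo_Surface is a goo surface actor that fills a spline-defined shape with instanced goo meshes.
; The construction script and UpdateBoxExtent both call CalculateMesh, which clears the instances and rebuilds them.
; MakeGridPoint turns the spline into grid vertices, and each one with a non-negative index gets a world-space instance with random, vertically flattened scale.
; BeginPlay, overlap and Tick only forward to the parent class.
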(event EventBeginPlay
  (|CallParentFunction))

(event Collision|EventActorBeginOverlap
  (params (OtherActor :type Actor%20Object%20Reference))
  (|CallParentFunction OtherActor))

(event EventTick
  (params (DeltaSeconds :type Float%20%28single-precision%29))
  (|CallParentFunction DeltaSeconds))

(fn ConstructionScript
  (|CallParentFunction)
  (CallFunction|CalculateMesh))

(fn UpdateBoxExtent
  (CallFunction|CalculateMesh))

(fn CalculateMesh
  (Components|InstancedStaticMesh|ClearInstances (Variables|Default|GetGoo_InstancedStaticMesh))
  (bind (_vertices _index) (CallFunction|MakeGridPoint (Variables|Default|GetSpline) 5e+01 100 1e+02 -2e+02))
  (for (_array_element _array_index) _vertices
    (if (>= (Utilities|Array|Get(acopy) _index _array_index) 0)
      (Components|InstancedStaticMesh|AddInstance (Variables|Default|GetGoo_InstancedStaticMesh) (Math|Transform|MakeTransform _array_element "0, 0, 0" (* (Math|Random|RandomFloatinRange 0.5 1.0) "1.000000,1.000000,0.500000")) true))))