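; BP_Fusil is a rifle pickup actor that the player collects by interacting with it.
; On Interact, it adds an AC_Fusil component to the interacting character and attaches it to the mesh's FusilSocket.
; It passes its MunitionsInitiales value to the component's Munitions, then destroys itself.
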(event EventBeginPlay
  (|CallParentFunction) ; This node is disabled and will not be called.\nDrag off pins to build functionality.
)

(event Collision|EventActorBeginOverlap
  (params (OtherActor :type Actor%20Object%20Reference))
  (|CallParentFunction OtherActor) ; This node is disabled and will not be called.\nDrag off pins to build functionality.
)

(event EventTick
  (params (DeltaSeconds :type Float%20%28single-precision%29))
  (|CallParentFunction DeltaSeconds) ; This node is disabled and will not be called.\nDrag off pins to build functionality.
)

(event EventInteract
  (params (ReferenceToCharacter :type BP%20Third%20Person%20Character%20Object%20Reference))
  (bind _returnvalue (Game|AddComponentbyClass ReferenceToCharacter "/Game/Blueprint/AC_Fusil.AC_Fusil_C" false))
  (Transformation|AttachComponentToComponent _returnvalue (Variables|/Script/Engine.Character|GetMesh ReferenceToCharacter) "FusilSocket" "KeepRelative" "KeepRelative" "KeepRelative" true)
  (Variables|/Game/Blueprint/AC_Fusil.AC_Fusil_C|SetMunitions _returnvalue (Variables|Default|GetMunitionsInitiales))
  (Actor|DestroyActor))

(fn ConstructionScript
  (|CallParentFunction))