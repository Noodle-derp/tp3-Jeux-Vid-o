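; BP_ReserveLait is an interactable milk reserve that refills a character's AC_HoseLait component.
; Overlap start and interaction require that component, and interaction calls its RemplirLait function.
; The result either stops the sound or triggers a DoOnce-gated Jump animation and pitched-down filling sound.
; Ending interaction restores the idle animation, stops the sound and resets the gate.
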(event EventBeginPlay
  (|CallParentFunction))

(event Collision|EventActorBeginOverlap
  (params (OtherActor :type Actor%20Object%20Reference))
  (Utilities|IsValid (Actor|GetComponentbyClass OtherActor "/Game/Blueprint/Lait/AC_HoseLait.AC_HoseLait_C")
    (:Is%20Valid
      (|CallParentFunction OtherActor))))

(event EventInteract
  (params (ReferenceToCharacter :type BP%20Third%20Person%20Character%20Object%20Reference))
  (bind _returnvalue (Actor|GetComponentbyClass ReferenceToCharacter "/Game/Blueprint/Lait/AC_HoseLait.AC_HoseLait_C"))
  (bind _skeletalmesh (Variables|Default|GetSkeletalMesh))
  (Utilities|IsValid _returnvalue
    (:Is%20Valid
      (bind _rempli_ (Default|RemplirLait _returnvalue))
      (if _rempli_
        (Utilities|IsValid (Variables|Default|GetSoundFX)
          (:Is%20Valid
            (Audio|Components|Audio|Stop (Variables|Default|GetSoundFX))
            (goto _label Reset))
          (:Is%20Not%20Valid
            (goto _label Reset)))
        (else
          (Utilities|FlowControl|DoOnce false :!label _label
            (:Completed
              (Components|Animation|SetAnimation _skeletalmesh "/Game/Fab/Cow/jump.jump")
              (Audio|Components|Audio|Play _skeletalmesh true)
              (bind _returnvalue_2 (Audio|SpawnSound2D "/Game/Audio/SFX/Filling.Filling" 0.25 0.125 1.0 0))
              (Variables|Default|SetSoundFX _returnvalue_2))))))))

(event EventEndInteract
  (bind _skeletalmesh (Variables|Default|GetSkeletalMesh))
  (bind _skeletalmesh_2 (Variables|Default|GetSkeletalMesh))
  (Components|Animation|SetAnimation _skeletalmesh "/Game/Fab/Cow/iddle.iddle")
  (Audio|Components|Audio|Play _skeletalmesh true)
  (Utilities|IsValid (Variables|Default|GetSoundFX)
    (:Is%20Valid
      (Audio|Components|Audio|Stop (Variables|Default|GetSoundFX))
      (Utilities|FlowControl|DoOnce false) ; enters at Reset
    )
    (:Is%20Not%20Valid
      (Utilities|FlowControl|DoOnce false) ; enters at Reset
    )))

(event Collision|EventActorEndOverlap
  (params (OtherActor :type Actor%20Object%20Reference))
  (|CallParentFunction OtherActor))

(fn ConstructionScript)