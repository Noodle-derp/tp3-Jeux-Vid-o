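; Infinite ammo refill point: an interactable that refills the interacting character's rifle without being used up.
; Interact looks up the character's AC_Fusil component and, if its ammo is not full, refills it by MunitionsMax and plays a reload sound.
; Sphere overlaps and Tick defer to the parent class.
; A separate AffichageTexte trigger shows the text render only while a BP_ThirdPersonCharacter overlaps it.
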(event OnComponentBeginOverlap(AffichageTexte)
  (params (OverlappedComponent :type Primitive%20Component%20Object%20Reference) (OtherActor :type Actor%20Object%20Reference) (OtherComp :type Primitive%20Component%20Object%20Reference) (OtherBodyIndex :type Integer) (bFromSweep :type Boolean) (SweepResult :type Hit%20Result%20Structure%20%28by%20ref%29))
  ;[0.15 0.15 0.15 0.5] Afficher le nombre de munition restant
  (Utilities|Casting|CastToBP_ThirdPersonCharacter OtherActor)
  (Rendering|SetVisibility (Variables|Default|GetTextRender_0) true false))

(event OnComponentEndOverlap(AffichageTexte)
  (params (OverlappedComponent :type Primitive%20Component%20Object%20Reference) (OtherActor :type Actor%20Object%20Reference) (OtherComp :type Primitive%20Component%20Object%20Reference) (OtherBodyIndex :type Integer))
  ;[0.15 0.15 0.15 0.5] Afficher le nombre de munition restant
  (Utilities|Casting|CastToBP_ThirdPersonCharacter OtherActor)
  (Rendering|SetVisibility (Variables|Default|GetTextRender_0) false false))

(event OnComponentBeginOverlap(Sphere)
  (params (OverlappedComponent :type Primitive%20Component%20Object%20Reference) (OtherActor :type Actor%20Object%20Reference) (OtherComp :type Primitive%20Component%20Object%20Reference) (OtherBodyIndex :type Integer) (bFromSweep :type Boolean) (SweepResult :type Hit%20Result%20Structure%20%28by%20ref%29))
  (|CallParentFunction OtherActor))

(event OnComponentEndOverlap(Sphere)
  (params (OverlappedComponent :type Primitive%20Component%20Object%20Reference) (OtherActor :type Actor%20Object%20Reference) (OtherComp :type Primitive%20Component%20Object%20Reference) (OtherBodyIndex :type Integer))
  (|CallParentFunction OtherActor))

(event EventTick
  (params (DeltaSeconds :type Float%20%28single-precision%29))
  (|CallParentFunction DeltaSeconds))

(event EventInteract
  (params (ReferenceToCharacter :type BP%20Third%20Person%20Character%20Object%20Reference))
  (bind _returnvalue (Actor|GetComponentbyClass ReferenceToCharacter "/Game/Blueprint/AC_Fusil.AC_Fusil_C"))
  (Utilities|IsValid _returnvalue
    (:Is%20Valid
      (bind _munitionspleines_ (Default|MunitionsPleines? _returnvalue))
      (if (not _munitionspleines_)
        (Default|RemplirMunitions _returnvalue (Variables|/Game/Blueprint/AC_Fusil.AC_Fusil_C|GetMunitionsMax _returnvalue))
        (Audio|PlaySound2D "/Game/Audio/SFX/Gun_Reload.Gun_Reload" 1.0 1.0 0.0 0 0)))))

(event Collision|EventActorBeginOverlap
  (params (OtherActor :type Actor%20Object%20Reference)))

(event Collision|EventActorEndOverlap
  (params (OtherActor :type Actor%20Object%20Reference)))

(fn ConstructionScript)